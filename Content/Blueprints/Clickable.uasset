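; Clickable is an unfinished Blueprint that adds mouse click and hover handling to its owning actor.
; On BeginPlay it binds the owner's click event, then caches a StaticMeshComponent and binds cursor-over only if one exists.
; Clicking toggles IsClicked, but the mesh response, hover handlers and OnClick function are empty, and the hover-end binding never runs.
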(event `self.ReceiveBeginPlay`
  (bind _returnvalue (`self.GetOwner`))
  (bind _returnvalue_2 (`self.GetComponentByClass` _returnvalue "/Script/Engine.StaticMeshComponent"))
  (add `self.OnClicked` _returnvalue (delegate `OnMouseClicked`))
  (`/Engine/EditorBlueprintResources/StandardMacros.IsValid` _returnvalue_2
    (:`Is Valid`
      (set `self.Static MeshRef` _returnvalue_2)
      (add `self.OnBeginCursorOver` _returnvalue (delegate `OnMouseHover`)))))

(event `OnMouseClicked` :!signature `self.OnClicked`
  (params (TouchedActor :type "Actor Object Reference") (ButtonPressed :type "Key Structure" :default "None"))
  (bind _output_get (set `self.isClicked` (not (`self.isClicked`))))
  (`/Engine/EditorBlueprintResources/StandardMacros.IsValid` (`self.Static MeshRef`)
    (:`Is Valid`
      (if _output_get
        _))))

(event `OnMouseHover` :!signature `self.OnBeginCursorOver`
  (params (TouchedActor :type "Actor Object Reference")))

(event `OnMouseHoverEnd` :!signature `self.OnEndCursorOver`
  (params (TouchedActor :type "Actor Object Reference")))

(fn `OnClick`)

(fn `UserConstructionScript`)