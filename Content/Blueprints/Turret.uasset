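; Auto-targeting twin-barrel turret that finds and shoots Enemy pawns within its sensing range.
; Each tick it picks the closest enemy with line of sight via a sphere overlap, then rotates the top mesh toward it at constant speed.
; Once the fire cooldown has elapsed and a dot-product check shows it facing the target, it spawns damage-carrying projectiles from the left, then right barrel sockets, slightly staggered.
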(event `self.ReceiveTick`
  (params (DeltaSeconds :type "Float (single-precision)"))
  (`self.Find Best Target`)
  (`self.Target`
    (:`then`
      (`self.UpdateTurretRotation` DeltaSeconds)
      (`self.Update Fire`))
    (:`else`)))

(event `Fire`
  (set `self.TimeOfLastFire` (`KismetSystemLibrary.GetGameTimeInSeconds`))
  (bind _returnvalue (`|SpawnActorFromClass` "/Script/MyProject2.Projectile" (`SceneComponent.GetSocketTransform` (`self.StaticMeshBarrelL`) "BulletSocket" "RTS_World") "Undefined" "OverrideRootScale" null null))
  (set `Projectile.baseDamage` (`self.Damage`) _returnvalue)
  (`KismetSystemLibrary.Delay` 0.2)
  (bind _returnvalue_2 (`|SpawnActorFromClass` "/Script/MyProject2.Projectile" (`SceneComponent.GetSocketTransform` (`self.StaticMeshBarrelR`) "BulletSocket" "RTS_World") "Undefined" "OverrideRootScale" self null))
  (set `Projectile.baseDamage` (`self.Damage`) _returnvalue_2)
  (`KismetSystemLibrary.Delay` 0.2))

(fn `Find Best Target`
  (locals (`BestDistance (local)` :type "Float (double-precision)") (`CurrentDistance (local)` :type "Float (double-precision)") (`BestTarget (local)` :type "Actor Object Reference") (`CurrentTarget (local)` :type "Actor Object Reference"))
  (set `local.BestDistance (local)` (+ (`self.SensingRange`) 1.0))
  (bind _outactors (`KismetSystemLibrary.SphereOverlapActors` (`self.K2_GetActorLocation`) (`self.SensingRange`) (`|MakeArray` "ObjectTypeQuery3" :!type "EObjectTypeQuery Enum") "/Game/Blueprints/Enemy.Enemy_C"))
  (for _array_element _outactors
    (bind _output_get (set `local.CurrentTarget (local)` _array_element))
    (bind _output_get_2 (set `local.CurrentDistance (local)` (`self.GetDistanceTo` _output_get self)))
    (if (or (< _output_get_2 (`local.BestDistance (local)`)) (not (`KismetSystemLibrary.IsValid` (`local.BestTarget (local)`))))
      (bind _result (`/Game/FunctionLibrary.Has Line Of Sight` (`SceneComponent.K2_GetComponentLocation` (`self.StaticMeshTop`)) (`self.K2_GetActorLocation` (`local.CurrentTarget (local)`)) (`|MakeArray` self (`local.CurrentTarget (local)`) :!type "Actor Object Reference")))
      (if _result
        (set `local.BestTarget (local)` (`local.CurrentTarget (local)`))
        (set `local.BestDistance (local)` (`local.CurrentDistance (local)`)))))
  (set `self.Target` (`local.BestTarget (local)`)))

(fn `Update Fire`
  (if (> (- (`KismetSystemLibrary.GetGameTimeInSeconds`) (`self.TimeOfLastFire`)) (`self.RateOfFire`))
    (if (> (`KismetMathLibrary.Dot_VectorVector` (`KismetMathLibrary.GetDirectionUnitVector` (`SceneComponent.K2_GetComponentLocation` (`self.StaticMeshTop`)) (`self.K2_GetActorLocation` (`self.Target`))) (`SceneComponent.GetForwardVector` (`self.StaticMeshTop`))) 0.98)
      (`self.Fire`))))

(fn `UpdateTurretRotation`
  (params (deltaSeconds :type "Float (double-precision)"))
  (`SceneComponent.K2_SetWorldRotation` (`self.StaticMeshTop`) (`KismetMathLibrary.RInterpTo_Constant` (`SceneComponent.K2_GetComponentRotation` (`self.StaticMeshTop`)) (`KismetMathLibrary.FindLookAtRotation` (`SceneComponent.K2_GetComponentLocation` (`self.StaticMeshTop`)) (`self.K2_GetActorLocation` (`self.Target`))) (`local.deltaSeconds`) (`self.Rotation Speed`)) false false))

(fn `UserConstructionScript`)