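; DefenceGameState is a game state Blueprint that tracks rounds, coins and game speed for a wave-based defence game.
; On BeginPlay it spawns a Spawner and binds to its round-complete event, which ends the round, resets game speed, then prints a win message or advances the round counter.
; StartNextRound switches on the current round to feed the Spawner, with only the first round wired.
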(event `self.ReceiveBeginPlay`
  (bind _returnvalue (`|SpawnActorFromClass` "/Game/Blueprints/Spawner.Spawner_C" (`self.Spawn Transform`) "Undefined" "OverrideRootScale" null null))
  (bind _output_get (set `self.Spawner` _returnvalue))
  (add `/Game/Blueprints/Spawner.Round Complete` _output_get (delegate `Round Complete`)))

(event `Round Complete`
  (bind _current_round (`self.Current Round`))
  (set `self.isRoundActive` false)
  (set `self.gameSpeed` "NewEnumerator0")
  (if (== _current_round (`self.Total Rounds`))
    (`KismetSystemLibrary.PrintString` "You Win")
    (else
      (`/Engine/EditorBlueprintResources/StandardMacros.IncrementInt` _current_round))))

(event `Start Next Round`
  (switch `int` (`self.Current Round`)
    (:`1`
      (`/Game/Blueprints/Spawner.Spawn Round` (`self.Spawner`) (`self.Round 1`)))))

(event `Add coins`
  (params (coins :type Integer))
  (set `self.Coins` (+ coins (`self.Coins`))))

(fn `UserConstructionScript`)