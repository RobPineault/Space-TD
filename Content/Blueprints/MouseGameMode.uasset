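; MouseGameMode is a game mode that tracks the player's Health and Coins and ends the game on defeat.
; Attacked decrements Health and calls StopGame when it reaches zero or below, while Addcoins adds to the coin total.
; StopGame pauses each Spawner's "spawn enemy" timer by function name and immediately halts every Enemy's character movement.
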(event `Attacked`
  (bind _result (`/Engine/EditorBlueprintResources/StandardMacros.DecrementInt` (`self.Health`))
    (:`  `
      (if (<= _result 0)
        (`self.Stop game`)))))

(event `Add coins`
  (params (coins :type Integer))
  (set `self.Coins` (+ coins (`self.Coins`))))

(event `Stop game`
  (bind _outactors (`GameplayStatics.GetAllActorsOfClass` "/Game/Blueprints/Spawner.Spawner_C"))
  (for _array_element _outactors
    (`KismetSystemLibrary.K2_PauseTimer` _array_element "spawn enemy"))
  (bind _outactors_2 (`GameplayStatics.GetAllActorsOfClass` "/Game/Blueprints/Enemy.Enemy_C"))
  (for _array_element_2 _outactors_2
    (`MovementComponent.StopMovementImmediately` (`Character.CharacterMovement` _array_element_2))))

(fn `UserConstructionScript`)