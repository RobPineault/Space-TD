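; Player character that flies freely, driven by axis input for orbiting, horizontal movement and vertical movement.
; BeginPlay sets CharacterMovement to Flying and prints whether that mode is active.
; CameraOrbit adds controller yaw scaled by OrbitSpeed.
; Forward and strafe input follow control yaw only, while up/down movement takes its up vector from control roll alone.
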(event `self.ReceiveBeginPlay`
  (`CharacterMovementComponent.SetMovementMode` (`self.CharacterMovement`) "MOVE_Flying" 0)
  (`KismetSystemLibrary.PrintString` (`KismetStringLibrary.Conv_BoolToString` (`NavMovementComponent.IsFlying` (`self.CharacterMovement`)))))

(event `CameraOrbit`
  (params (Magnitude :type "Float (double-precision)"))
  (`self.AddControllerYawInput` (* Magnitude (`self.orbit speed`))))

(event `MoveForward`
  (params (Magnitude :type "Float (double-precision)"))
  (`self.AddMovementInput` (`KismetMathLibrary.GetForwardVector` (`KismetMathLibrary.MakeRotator` 0.0 0.0 (.yaw (`self.GetControlRotation`)))) Magnitude))

(event `LeftRightStrafe`
  (params (Magnitude :type "Float (double-precision)"))
  (`self.AddMovementInput` (`KismetMathLibrary.GetRightVector` (`KismetMathLibrary.MakeRotator` 0.0 0.0 (.yaw (`self.GetControlRotation`)))) Magnitude))

(event `UpDownStrafe`
  (params (Magnitude :type "Float (double-precision)"))
  (`self.AddMovementInput` (`KismetMathLibrary.GetUpVector` (`KismetMathLibrary.MakeRotator` (.roll (`self.GetControlRotation`)))) Magnitude))

(fn `UserConstructionScript`)