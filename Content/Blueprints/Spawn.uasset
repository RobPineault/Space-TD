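; Spawner actor that spawns a set number of AI pawns of a given class at its location on a repeating timer.
; StartSpawning stores the count and class and starts the looping timer, which is cleared once the count is reached.
; Only the final spawn's Killed event is bound; when it fires, the actor calls Finished and destroys itself, regardless of whether earlier spawns are still alive.
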(event `Start Spawning`
  (params (Total :type Integer) (Interval :type "Float (double-precision)") (Enemy :type "/Game/Blueprints/Enemy Class Reference"))
  (set `self.Total` Total)
  (set `self.Enemy` Enemy)
  (bind _returnvalue (`KismetSystemLibrary.K2_SetTimerDelegate` (delegate `Spawn`) Interval true)))

(event `Spawn`
  (bind _returnvalue (`AIBlueprintHelperLibrary.SpawnAIFromClass` (`self.Enemy`) null (`self.K2_GetActorLocation`) (struct) true null))
  (bind _result (`/Engine/EditorBlueprintResources/StandardMacros.IncrementInt` (`self.Spawn Count`))
    (:`  `
      (if (== (`self.Total`) _result)
        (`KismetSystemLibrary.K2_ClearAndInvalidateTimerHandle` (stale `Start Spawning` _returnvalue))
        (bind _asenemy (cast `/Game/Blueprints/Enemy` _returnvalue))
        (add `/Game/Blueprints/Enemy.Killed` _asenemy (delegate `LastKilled`))))))

(event `LastKilled`
  (`self.Finished`)
  (`self.K2_DestroyActor`))

(fn `UserConstructionScript`)