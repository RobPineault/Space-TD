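; Player controller that handles mouse-driven building placement and forwards orbit, move and height-limited up/down input to the Player pawn.
; SetPlaceableData stores the selected building's classes and cost, and enabling placement mode spawns a preview actor.
; Each tick a cursor line trace moves the preview.
; Left click checks validity, purchases through DefensePlayerState, spawns the building, exits placement mode and fires Placed with the button index.
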(event `self.ReceiveBeginPlay`
  (bind _asdefense_player_state (cast `/Game/Blueprints/DefensePlayerState` (`self.PlayerState`)))
  (set `self.PlayerStateRef` _asdefense_player_state)
  (`self.SetControlRotation` (`KismetMathLibrary.MakeRotator` 0.0 0.0 90.0)))

(event `self.ReceiveTick`
  (params (DeltaSeconds :type "Float (single-precision)"))
  (if (`self.PlacementModeEnabled`)
    (`self.UpdatePlacement`)))

(event `InputAction|MouseLeftClick`
  (params (Key :type "Key Structure"))
  (:`Pressed`
    (if (`self.PlacementModeEnabled`)
      (`self.SpawnBuilding`))))

(event `InputAxis|Orbit`
  (params (AxisValue :type "Float (single-precision)"))
  (bind _asplayer (cast `/Game/Blueprints/Player` (`self.K2_GetPawn`)))
  (`/Game/Blueprints/Player.CameraOrbit` _asplayer AxisValue))

(event `InputAxis|MoveForward`
  (params (AxisValue :type "Float (single-precision)"))
  (bind _asplayer (cast `/Game/Blueprints/Player` (`self.K2_GetPawn`)))
  (`/Game/Blueprints/Player.MoveForward` _asplayer AxisValue))

(event `InputAxis|MoveRight`
  (params (AxisValue :type "Float (single-precision)"))
  (bind _asplayer (cast `/Game/Blueprints/Player` (`self.K2_GetPawn`)))
  (`/Game/Blueprints/Player.LeftRightStrafe` _asplayer AxisValue))

(event `InputAxis|UpDown`
  (params (AxisValue :type "Float (single-precision)"))
  (bind _asplayer (cast `/Game/Blueprints/Player` (`self.K2_GetPawn`)))
  (if (< AxisValue 1.0)
    (bind _z (.z (`CharacterMovementComponent.GetLastUpdateLocation` (`Character.CharacterMovement` _asplayer))))
    (if (> _z (`self.Min Height`))
      (`/Game/Blueprints/Player.UpDownStrafe` _asplayer AxisValue :!label _label))
    (elif (< _z (`self.Max Height`))
      (goto _label))))

(fn `Set Placeable Data`
  (params (PlaceableData :type "/Game/Blueprints/PlaceableStruct Structure") (ButtonIndex :type Integer))
  (bind (_spawnactor _previewactor _cost) (break `/Game/Blueprints/PlaceableStruct` PlaceableData))
  (set `self.PlaceableActorType` _spawnactor)
  (set `self.ActorPreviewType` _previewactor)
  (set `self.Cost` _cost)
  (set `self.PlaceableButtonIndex` ButtonIndex)
  (return))

(fn `SetPlacementModeEnabled`
  (params (isEnabled :type Boolean))
  (bind _placeableactor (`self.PlaceableActor`))
  (if (== isEnabled (`self.PlacementModeEnabled`))
    (return)
    (else
      (bind _output_get (set `self.PlacementModeEnabled` isEnabled))
      (if _output_get
        (bind _returnvalue (`|SpawnActorFromClass` (`self.ActorPreviewType`) (`KismetMathLibrary.MakeTransform` (0.0 0.0 -100000000.0)) "AlwaysSpawn" "OverrideRootScale" null null))
        (bind _output_get_2 (set `self.PlaceableActor` _returnvalue))
        (bind _returnvalue_2 (`self.GetComponentByClass` _output_get_2 "/Game/Blueprints/Clickable_Component.Clickable_Component_C"))
        (`/Engine/EditorBlueprintResources/StandardMacros.IsValid` _returnvalue_2
          (:`Is Valid`
            (`/Game/Blueprints/Clickable_Component.inPlacementMode` _returnvalue_2))
          (:`Is Not Valid`
            _))
        (`AddComponent|NODE_AddPlaceableComponent-0` :`self` _output_get_2)
        (else
          (`/Engine/EditorBlueprintResources/StandardMacros.IsValid` _placeableactor
            (:`Is Valid`
              (`self.K2_DestroyActor` _placeableactor))))))))

(fn `SpawnBuilding`
  (bind _returnvalue (`self.GetComponentByClass` (`self.PlaceableActor`) "/Game/Blueprints/PlaceableComponent.PlaceableComponent_C"))
  (`/Engine/EditorBlueprintResources/StandardMacros.IsValid` _returnvalue
    (:`Is Valid`
      (if (`/Game/Blueprints/PlaceableComponent.isPlacementValid` _returnvalue)
        (bind _successful (`/Game/Blueprints/DefensePlayerState.Purchase` (`self.PlayerStateRef`) (`self.Cost`)))
        (if _successful
          (`|SpawnActorFromClass` (`self.PlaceableActorType`) (`self.GetTransform` (`self.PlaceableActor`)) "AlwaysSpawn" "OverrideRootScale" null null)
          (`self.SetPlacementModeEnabled` false)
          (`self.Placed` (`self.PlaceableButtonIndex`)))))))

(fn `UpdatePlacement`
  (bind (_worldlocation _worlddirection) (`self.DeprojectMousePositionToWorld`))
  (bind _outhit (`KismetSystemLibrary.LineTraceSingle` _worldlocation (+ _worlddirection (* _worlddirection 50000.0)) "TraceTypeQuery3"))
  (bind (_bblockinghit _binitialoverlap _time _distance _location) (`GameplayStatics.BreakHitResult` _outhit))
  (if _bblockinghit
    (`self.K2_SetActorLocation` (`self.PlaceableActor`) _location false false)))

(fn `UserConstructionScript`)