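; DefensePlayerState is a player state Blueprint that holds a player's Coins balance, apparently for a defense game.
; The Addcoins event increases the balance.
; The Purchase function checks the balance against a cost, deducts it when affordable, and returns whether the purchase succeeded.
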(event `Add coins`
  (params (coins :type Integer))
  (set `self.Coins` (+ coins (`self.Coins`))))

(fn `Purchase`
  (params (Cost :type Integer))
  (returns (Successful :type Boolean))
  (bind _coins (`self.Coins`))
  (if (>= _coins Cost)
    (set `self.Coins` (- _coins Cost))
    (return true)
    (else
      (return false))))

(fn `UserConstructionScript`)