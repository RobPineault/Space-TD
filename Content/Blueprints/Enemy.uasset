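; Base enemy for a defense game that walks to a target point, damages the player's side on arrival, and awards coins when killed.
; ParentBeginPlay receives health and coin value, initializes the widget health bar, then uses AI MoveTo toward the first TargetPoint found, notifying DefenseGameMode on success.
; TakeDamage clamps health, updates the bar, and at zero destroys the enemy, pays coins and calls Killed.
; PredictLocation requests an AI prediction event for its future position.
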(event `Parent BeginPlay`
  (params (Enemy :type "Pawn Object Reference") (Health :type "Float (double-precision)") (Value :type Integer))
  (bind _maxenemyhealth (`self.maxEnemyHealth`))
  (`KismetSystemLibrary.Delay` 0.1)
  (set `self.maxEnemyHealth` Health)
  (set `self.enemyHealth` Health)
  (set `self.value` Value)
  (bind _ashealth_bar (cast `/Game/Blueprints/Health_Bar` (`WidgetComponent.GetUserWidgetObject` (`self.HealthWC`))))
  (set `/Game/Blueprints/Health_Bar.maxHealth` _maxenemyhealth _ashealth_bar)
  (set `/Game/Blueprints/Health_Bar.health` _maxenemyhealth _ashealth_bar)
  (bind _outactors (`GameplayStatics.GetAllActorsOfClass` "/Script/Engine.TargetPoint"))
  (`|AIMoveTo` Enemy (0.0 0.0 0.0) (`|GetArrayItem` _outactors)
    (:`OnSuccess`
      (bind _asdefense_game_mode (cast `/Game/Blueprints/DefenseGameMode` (`GameplayStatics.GetGameMode`)))
      (`/Game/Blueprints/DefenseGameMode.Attacked` _asdefense_game_mode)
      (`self.K2_DestroyActor`))))

(event `Take Damage`
  (params (damage :type "Float (double-precision)"))
  (bind _currenthealth (`self.Modify Health` damage))
  (bind _ashealth_bar (cast `/Game/Blueprints/Health_Bar` (`WidgetComponent.GetUserWidgetObject` (`self.HealthWC`))))
  (`/Game/Blueprints/Health_Bar.Update Health` _ashealth_bar _currenthealth)
  (if (== 0.0 _currenthealth)
    (`self.K2_DestroyActor`)
    (bind _asmouse_player_controller (cast `/Game/Blueprints/mousePlayerController` (`GameplayStatics.GetPlayerController` 0)))
    (`/Game/Blueprints/DefensePlayerState.Add coins` (`/Game/Blueprints/mousePlayerController.PlayerStateRef` _asmouse_player_controller) (`self.value`))
    (`self.Killed`)))

(fn `Modify Health`
  (params (healthToSubtract :type "Float (double-precision)"))
  (returns (currentHealth :type "Float (double-precision)"))
  (bind _output_get (set `self.enemyHealth` (`KismetMathLibrary.FClamp` (- (`self.enemyHealth`) healthToSubtract) 0.0 (`self.maxEnemyHealth`))))
  (return _output_get))

(fn `NewFunction_0`
  (set `self.maxEnemyHealth` (`self.enemyHealth`)))

(fn `Predict location`
  (params (time :type "Float (double-precision)"))
  (`AISense_Prediction.RequestControllerPredictionEvent` (`AIBlueprintHelperLibrary.GetAIController` self) self time))

(fn `UserConstructionScript`)