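; Spawner actor that runs an enemy round from an array of spawn data and signals when the round is complete.
; SpawnRound creates a Spawn actor per entry, passing count, interval and enemy class, with a delay between entries.
; The last one's Finished event triggers while loops that poll, without delays, until no Spawn or Enemy actors remain, then RoundComplete is called.
; A SpawnEnemy helper spawns AI at the spawner's location.
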(event `Spawn Round`
  (params (`Spawn Data` :type "Array of /Game/Blueprints/SpawnBatch Structure"))
  (set `self.Spawning Enemies` true)
  (bind (_array_element _array_index) (`/Engine/EditorBlueprintResources/StandardMacros.For Each Loop Wait` `Spawn Data` :!label _label)
    (:`Loop Body`
      (bind _returnvalue (`|SpawnActorFromClass` "/Game/Blueprints/Spawn.Spawn_C" (`self.GetTransform`) "AlwaysSpawn" "OverrideRootScale" null null))
      (if (== (- (`KismetArrayLibrary.Array_Length` `Spawn Data`) 1) _array_index)
        (add `/Game/Blueprints/Spawn.Finished` _returnvalue (delegate `Finish Spawning`)))
      (bind (_total _interval _delay _enemyclass) (break `/Game/Blueprints/SpawnBatch` _array_element))
      (`/Game/Blueprints/Spawn.Start Spawning` _returnvalue _total _interval _enemyclass)
      (`KismetSystemLibrary.Delay` _delay)
      (goto _label :!via `Next Body`))))

(event `Finish Spawning`
  (while (> (`KismetArrayLibrary.Array_Length` (stale _outactors)) 0)
    (bind _outactors (`GameplayStatics.GetAllActorsOfClass` "/Game/Blueprints/Spawn.Spawn_C")))
  (while (> (`KismetArrayLibrary.Array_Length` (stale _outactors_2)) 0)
    (bind _outactors_2 (`GameplayStatics.GetAllActorsOfClass` "/Game/Blueprints/Enemy.Enemy_C")))
  (`self.Round Complete`))

(fn `Spawn Enemy`
  (params (Enemy :type "/Game/Blueprints/Enemy Class Reference"))
  (`AIBlueprintHelperLibrary.SpawnAIFromClass` Enemy null (`self.K2_GetActorLocation`) (struct) true null))

(fn `UserConstructionScript`)