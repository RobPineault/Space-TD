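; Clickable actor component that lets its owner toggle a selected look by click and flags it for custom depth on hover.
; A custom event binds the owner's cursor events and caches its static mesh, whose first material swaps between Active and BaseMaterial.
; The hover-end binding is unconnected, so custom depth stays on once set.
; An inPlacementMode event destroys the component, and the Start/End Mouse Over functions are empty.
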(event `CustomEvent`
  (bind _returnvalue (`self.GetOwner`))
  (bind _returnvalue_2 (`Actor.GetComponentByClass` _returnvalue "/Script/Engine.StaticMeshComponent"))
  (add `Actor.OnClicked` _returnvalue (delegate `OnMouseClicked`))
  (`/Engine/EditorBlueprintResources/StandardMacros.IsValid` _returnvalue_2
    (:`Is Valid`
      (set `self.Static MeshRef` _returnvalue_2)
      (add `Actor.OnBeginCursorOver` _returnvalue (delegate `OnMouseHover`)))))

(event `OnMouseClicked`
  (params (TouchedActor :type "Actor Object Reference") (ButtonPressed :type "Key Structure"))
  (bind _static_meshref (`self.Static MeshRef`))
  (bind _output_get (set `self.isClicked` (not (`self.isClicked`))))
  (`/Engine/EditorBlueprintResources/StandardMacros.IsValid` (`self.Static MeshRef`)
    (:`Is Valid`
      (if _output_get
        (`PrimitiveComponent.SetMaterial` _static_meshref 0 "/Game/materials/Active.Active")
        (else
          (`PrimitiveComponent.SetMaterial` _static_meshref 0 "/Game/TwinStick/Meshes/BaseMaterial.BaseMaterial"))))))

(event `OnMouseHover`
  (params (TouchedActor :type "Actor Object Reference"))
  (`PrimitiveComponent.SetRenderCustomDepth` (`self.Static MeshRef`) true))

(event `OnMouseHoverEnd`
  (params (TouchedActor :type "Actor Object Reference"))
  (`PrimitiveComponent.SetRenderCustomDepth` (`self.Static MeshRef`) false))

(event `inPlacementMode`
  (`self.K2_DestroyComponent`))

(fn `End Mouse Over`)

(fn `Start Mouse Over`)