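; Actor component that shows whether its owning actor can be placed at its current position.
; It binds to the owner's begin and end overlap events and re-evaluates on each, as well as on BeginPlay.
; Placement counts as valid only when the owner overlaps no other actors.
; The result is stored in IsPlacementValid and swaps the first material slot of every static mesh on the owner between valid and invalid materials.
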(event `self.ReceiveBeginPlay`
  (bind _returnvalue (`self.GetOwner`))
  (add `Actor.OnActorBeginOverlap` _returnvalue (delegate `OverlapStateChanged`))
  (add `Actor.OnActorEndOverlap` _returnvalue (delegate `OverlapStateChanged`))
  (`self.UpdateState`))

(event `OverlapStateChanged`
  (params (OverlappedActor :type "Actor Object Reference") (OtherActor :type "Actor Object Reference"))
  (`self.UpdateState`))

(fn `UpdateState`
  (bind _output_get (set `self.isPlacementValid` (== (`KismetArrayLibrary.Array_Length` (`Actor.GetOverlappingActors` (`self.GetOwner`) "/Script/Engine.Actor")) 0)))
  (for _array_element (`Actor.K2_GetComponentsByClass` (`self.GetOwner`) "/Script/Engine.StaticMeshComponent")
    (if _output_get
      (`PrimitiveComponent.SetMaterial` _array_element 0 (`self.PlaceableMaterial`))
      (else
        (`PrimitiveComponent.SetMaterial` _array_element 0 (`self.InvalidPlaceableMaterial`))))))